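; BP_Soldier_01 is an unfinished soldier pawn that moves along fixed world axes: left/right on X, forward/backward on Y.
; Tick calls UpdateRotation, but that function is empty.
; Its disconnected nodes would set control yaw from the direction of mouse velocity, derived from mouse delta over delta time.
; MouseVelocity and IsDeadZone, a speed-above-threshold test, are likewise unwired, so only movement input takes effect.
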(event EventTick
  (params (DeltaSeconds :type Float%20%28single-precision%29))
  (CallFunction|UpdateRotation))

(event Input|AxisEvents|InputAxisMoveForwardBackwards
  (params (AxisValue :type Float%20%28single-precision%29))
  (Pawn|Input|AddMovementInput "0,1.000000, 0" AxisValue false))

(event Input|AxisEvents|InputAxisMoveLeftRight
  (params (AxisValue :type Float%20%28single-precision%29))
  (Pawn|Input|AddMovementInput "1.000000, 0, 0" AxisValue false))

(fn ConstructionScript)

(fn UpdateRotation)

(fn MouseVelocity)

(fn IsDeadZone)